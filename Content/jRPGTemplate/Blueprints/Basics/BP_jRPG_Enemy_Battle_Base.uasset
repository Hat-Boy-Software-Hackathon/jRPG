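; Base enemy combatant Blueprint for battles in the jRPG template, handling what happens when an enemy dies.
; Its OnDeath event sets the Dead flag, stops the current animation montage and, if the battle manager reference is valid, reports itself through OnEnemyKilled.
; The construction script only calls its parent, and the BeginPlay and overlap events are disabled stubs.
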(event `/Game/jRPGTemplate/Blueprints/Interfaces/BPI_BattleCommunication.OnDeath`
  (set `self.Dead?` true)
  (bind _returnvalue (`self.GetCurrentMontage`))
  (`self.StopAnimMontage` _returnvalue)
  (bind _battlemanagerreference (`self.BattleManagerReference`)
    (:`then`
      (`/Game/jRPGTemplate/Blueprints/Components/AC_jRPG_BattleManager.OnEnemyKilled` _battlemanagerreference self))
    (:`else`)))

(fn `UserConstructionScript`
  (`parent.UserConstructionScript`))